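; Door actor that opens for a player who has collected a key.
; On overlap it casts the other actor to ThirdPersonCharacter and checks its HasCollectedKey flag.
; If the flag is set and the door is still closed, it destroys the Box1 and SMDoor components and sets DoorOpened, so the door stays open.
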(event `self.ReceiveBeginPlay`
  (set `self.doorOpened` false))

(event `self.ReceiveActorBeginOverlap`
  (params (OtherActor :type "Actor Object Reference"))
  (bind _asthird_person_character (cast `/Game/ThirdPersonBP/Blueprints/ThirdPersonCharacter` OtherActor))
  (if (`/Game/ThirdPersonBP/Blueprints/ThirdPersonCharacter.hasCollectedKey` _asthird_person_character)
    (if (not (`self.doorOpened`))
      (`ActorComponent.K2_DestroyComponent` (`self.Box1`))
      (`ActorComponent.K2_DestroyComponent` (`self.SM_Door`))
      (set `self.doorOpened` true))))

(fn `UserConstructionScript`)